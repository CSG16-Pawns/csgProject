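; CatapultChargingSceneComp_snow is a component that charges a catapult's shot power and shows it on screen.
; Initialize sets the catapult's CurrentPower to a base value, adds a CatapultChargingBar widget to the viewport and enables tick.
; Each tick raises the power over time, maps it onto the bar's slider and calls ForcedFire on the catapult once it exceeds the maximum.
; Die removes the bar and destroys the component.
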(event `Initialize`
  (params (MyCatapult :type "/Game/Blueprints/Catapult Object Reference"))
  (set `self.MyCatapult` MyCatapult)
  (set `/Game/Blueprints/Catapult.CurrentPower` (`self.BasePower`) (`self.MyCatapult`))
  (bind _returnvalue (`|CreateWidget` "/Game/Blueprints/CatapultChargingBar.CatapultChargingBar_C"))
  (bind _output_get (set `self.Slider` _returnvalue))
  (`UserWidget.AddToViewport` _output_get 0)
  (`self.SetComponentTickEnabled` true))

(event `self.ReceiveBeginPlay`)

(event `Die`
  (`Widget.RemoveFromParent` (`self.Slider`))
  (`self.K2_DestroyComponent`))

(event `self.ReceiveTick`
  (params (DeltaSeconds :type "Float (single-precision)"))
  (bind _mycatapult (`self.MyCatapult`))
  (bind _output_get (set `/Game/Blueprints/Catapult.CurrentPower` (+ (`/Game/Blueprints/Catapult.CurrentPower` _mycatapult) (* DeltaSeconds (`self.PowerBuildSpeed`))) _mycatapult))
  (`Slider.SetValue` (`/Game/Blueprints/CatapultChargingBar.Slider_49` (`self.Slider`)) (`KismetMathLibrary.MapRangeClamped` _output_get (`self.BasePower`) (`self.MaxPower`) 0.0 1.0))
  (if (> _output_get (`self.MaxPower`))
    (`/Game/Blueprints/Catapult.ForcedFire` (`self.MyCatapult`))))