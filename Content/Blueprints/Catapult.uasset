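; Player-fired catapult that charges while Fire is held and launches a projectile on release, followed by a cooldown.
; Pressing Fire adds a charging component initialized with the catapult; releasing kills it, as does ForcedFire, which shares the launch path.
; A timeline swings the pivot's pitch, then after a short delay CatapultProjectile spawns with CurrentPower as speed, power resets and the swing reverses.
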(event `CatapultCooldown`
  (set `self.OffCooldown` false)
  (`KismetSystemLibrary.Delay` (`self.CooldownTime`))
  (set `self.OffCooldown` true))

(event `InputAction|Fire`
  (params (Key :type "Key Structure" :default "AnyKey"))
  (bind _projectiletransform (`self.ProjectileTransform`))
  (bind _offcooldown (`self.OffCooldown`))
  (:`Pressed`
    (if (and _offcooldown (not (`self.IsFiring`)))
      (set `self.IsFiring` true)
      (bind _returnvalue (`AddComponent|Catapult Charging Scene Comp Snow_1`))
      (bind _output_get (set `self.MyCharging` _returnvalue))
      (`/Game/Blueprints/CatapultChargingSceneComp_snow.Initialize` _output_get self)))
  (:`Released`
    (if (and _offcooldown (`self.IsFiring`)) :!label _label
      (set `self.IsFiring` false)
      (`/Game/Blueprints/CatapultChargingSceneComp_snow.Die` (`self.MyCharging`))
      (`self.CatapultCooldown`)
      (`|ExecutionSequence`
        (:`then_0`
          (bind (_direction _rotation) (`Timeline|FireThatShit` :!label _label_2)
            (:`Update`
              (`SceneComponent.K2_SetRelativeRotation` (`self.PivotForRotation`) (`KismetMathLibrary.MakeRotator` 0.0 _rotation) false false))))
        (:`then_1`
          (`KismetSystemLibrary.Delay` 0.2)
          (`|SpawnActorFromClass` "/Game/Blueprints/CatapultProjectile.CatapultProjectile_C" (`KismetMathLibrary.MakeTransform` (`SceneComponent.K2_GetComponentLocation` _projectiletransform) (`SceneComponent.K2_GetComponentRotation` _projectiletransform)) "Undefined" "OverrideRootScale" null (`self.CurrentPower`))
          (set `self.CurrentPower` 0.0)
          (goto _label_2 :!via `Reverse`))))))

(event `ForcedFire`
  (goto _label))

(event `self.ReceiveTick`
  (params (DeltaSeconds :type "Float (single-precision)")))

(fn `UserConstructionScript`)