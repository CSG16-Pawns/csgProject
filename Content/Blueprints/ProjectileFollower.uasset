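; Camera rig that follows a projectile, with a spring arm that the look inputs rotate.
; Initialize stores the projectile, and Tick moves the actor to its location without sweeping while it remains valid.
; Both look axes share one update that adjusts stored pitch and yaw and applies them as the spring arm's relative rotation.
; BeginPlay only prints a server or client debug message, and the unpossess event is an empty stub.
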(event `InputAxis|A_LookUp_Down`
  (params (AxisValue :type "Float (single-precision)"))
  (bind (_rotation_roll _rotation_pitch _rotation_yaw) (`KismetMathLibrary.BreakRotator` (`self.Rotation`)))
  (bind _output_get (set `self.Rotation` (`KismetMathLibrary.MakeRotator` 0.0 (+ _rotation_pitch (* AxisValue -1.0)) (+ _rotation_yaw (stale `InputAxis|A_LookRight_Left` AxisValue))) :!label _label))
  (`SceneComponent.K2_SetRelativeRotation` (`self.SpringArm`) _output_get false false))

(event `InputAxis|A_LookRight_Left`
  (params (AxisValue :type "Float (single-precision)"))
  (goto _label))

(event `UnpossessShit`)

(event `self.ReceiveBeginPlay`
  (`/Engine/EditorBlueprintResources/ActorMacros.Switch Has Authority`
    (:`Authority`
      (`KismetSystemLibrary.PrintString` "hi im the server"))
    (:`Remote`
      (`KismetSystemLibrary.PrintString` "hi im the client"))))

(event `Initialize`
  (params (ProjectileToFollow :type "/Game/Blueprints/Missiles/BasicProjectile Object Reference"))
  (set `self.ProjectileToFollow` ProjectileToFollow))

(event `self.ReceiveTick`
  (params (DeltaSeconds :type "Float (single-precision)"))
  (bind _projectiletofollow (`self.ProjectileToFollow`))
  (if (`KismetSystemLibrary.IsValid` _projectiletofollow)
    (`self.K2_SetActorLocation` (`self.K2_GetActorLocation` _projectiletofollow))))

(fn `UserConstructionScript`)