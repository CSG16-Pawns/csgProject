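; CatapultProjectile is a catapult projectile pawn that player controller 0 possesses when it begins play.
; The construction script copies Speed into ProjectileMovement's initial speed.
; Both look axes share one path that adds roll and yaw to the SpringArm, then re-sets actor rotation from its current roll and yaw.
; Logic to grow the sphere and gravity scale over time is disconnected, and Tick is empty.
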(event `self.ChildCollision`)

(event `InputAxis|A_LookUp_Down`
  (params (AxisValue :type "Float (single-precision)"))
  (bind (_returnvalue_roll _returnvalue_pitch _returnvalue_yaw) (`KismetMathLibrary.BreakRotator` (`self.K2_GetActorRotation`)))
  (`SceneComponent.K2_AddWorldRotation` (`self.SpringArm`) (`KismetMathLibrary.MakeRotator` AxisValue 0.0 (stale `InputAxis|A_LookRight_Left` AxisValue)) false false :!label _label)
  (`self.K2_SetActorRotation` (`KismetMathLibrary.MakeRotator` _returnvalue_roll 0.0 _returnvalue_yaw)))

(event `InputAxis|A_LookRight_Left`
  (params (AxisValue :type "Float (single-precision)"))
  (goto _label))

(event `self.ReceiveBeginPlay`
  (`Controller.Possess` (`GameplayStatics.GetPlayerController` 0) self))

(event `self.ReceiveTick`
  (params (DeltaSeconds :type "Float (single-precision)")))

(fn `UserConstructionScript`
  (set `ProjectileMovementComponent.InitialSpeed` (`self.Speed`) (`self.ProjectileMovement`)))