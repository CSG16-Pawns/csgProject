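; Base missile projectile that, on hitting a BaseDestructible, has a random HitChance to fracture destructible components around the impact.
; The server forwards hits through MulticastHit, so each receiving machine rolls the chance itself.
; Radius damage hits the struck component and ExplosionSphere's overlapping destructibles, using sphere radius as damage and impact speed for impulse.
; An empty ChildCollision hook, called per overlapping destructible, lets subclasses add behavior.
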(event `MulticastHit`
  (params (MyComp :type "PrimitiveComponent Object Reference") (Other :type "Actor Object Reference") (OtherComp :type "PrimitiveComponent Object Reference") (SelfMoved :type Boolean) (HitLocation :type "Vector Structure") (HitNormal :type "Vector Structure") (HitImpulse :type "Vector Structure") (Hit :type "HitResult Structure"))
  (bind _sphereradius (`SphereComponent.SphereRadius` (`self.ExplosionSphere`)))
  (if (<= (`KismetMathLibrary.RandomFloatInRange` 0.0 1.0) (`self.HitChance`))
    (cast `/Game/Blueprints/Destructible/BaseDestructible` Other)
    (bind _asdestructible_component (cast `DestructibleComponent` OtherComp))
    (bind _returnvalue (`PrimitiveComponent.GetPhysicsLinearVelocity` MyComp "None"))
    (for _array_element (`PrimitiveComponent.GetOverlappingComponents` (`self.ExplosionSphere`))
      (bind _asdestructible_component_2 (cast `DestructibleComponent` _array_element))
      (`DestructibleComponent.ApplyRadiusDamage` _asdestructible_component _sphereradius HitLocation _sphereradius (* (`KismetMathLibrary.VSize` _returnvalue) 20.0) false)
      (`DestructibleComponent.ApplyRadiusDamage` _asdestructible_component_2 _sphereradius HitLocation _sphereradius (* (`KismetMathLibrary.VSize` _returnvalue) 20.0) false)
      (`self.ChildCollision`))))

(event `self.ReceiveHit`
  (params (MyComp :type "PrimitiveComponent Object Reference") (Other :type "Actor Object Reference") (OtherComp :type "PrimitiveComponent Object Reference") (bSelfMoved :type Boolean) (HitLocation :type "Vector Structure") (HitNormal :type "Vector Structure") (NormalImpulse :type "Vector Structure") (Hit :type "HitResult Structure (by ref)"))
  (`/Engine/EditorBlueprintResources/ActorMacros.Switch Has Authority`
    (:`Authority`
      (`self.MulticastHit` MyComp Other OtherComp bSelfMoved HitLocation HitNormal NormalImpulse Hit))))

(event `ChildCollision`)

(fn `UserConstructionScript`)