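; Base Blueprint for destructible objects made of several DestructibleComponents that share one health pool.
; ApplyHitDamage subtracts from HealthPoints and damages only the hit component while health remains.
; At zero health it damages the root's direct destructible children at their own locations with half impulse strength, stopping at any non-destructible child.
; PartIsDestroyed checks DestroyedParts but returns true for absent parts and only adds parts already listed.
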(fn `ApplyHitDamage`
  (params (Damage :type Integer) (location :type "Vector Structure") (direction :type "Vector Structure") (strenght :type "Float (double-precision)") (hitDestructible :type "DestructibleComponent Object Reference"))
  (bind _output_get (set `self.HealthPoints` (- (`self.HealthPoints`) Damage)))
  (if (<= _output_get 0)
    (for _array_element (`SceneComponent.GetChildrenComponents` (`self.DefaultSceneRoot`) false)
      (bind _asdestructible_component (cast `DestructibleComponent` _array_element))
      (`DestructibleComponent.ApplyDamage` _asdestructible_component 1.0 (`SceneComponent.K2_GetComponentLocation` _asdestructible_component) direction (/ strenght 2.0)))
    (return)
    (else
      (`DestructibleComponent.ApplyDamage` hitDestructible 1.0 location direction strenght)
      (return))))

(fn `PartIsDestroyed`
  (params (part :type "DestructibleComponent Object Reference"))
  (returns (destroyed :type Boolean))
  (if (`KismetArrayLibrary.Array_Contains` (`self.DestroyedParts`) part)
    (`KismetArrayLibrary.Array_Add` (`self.DestroyedParts`) part)
    (return false)
    (else
      (return true))))

(fn `UserConstructionScript`)