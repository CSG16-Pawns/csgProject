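; Physics-driven arrow pawn that launches along its stem's forward vector when Shoot is called.
; The head welds to the stem at BeginPlay, and the construction script offsets the stem's center of mass using a CenterOfMass component's relative location.
; Shoot enables stem physics and applies an impulse scaled by MagnusPowerStrengthMeter.
; Debug arrow drawing, a gamepad test trigger and a head mass override remain disconnected.
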(event `self.ReceiveBeginPlay`
  (`SceneComponent.K2_AttachToComponent` (`self.Arrow_Head`) (`self.Arrow_Stem`) "None" "KeepWorld" "KeepWorld" "KeepWorld" true))

(event `self.ReceiveTick`
  (params (DeltaSeconds :type "Float (single-precision)")))

(fn `Shoot`
  ;[1 1 1] Activate physics behaviour
  (`PrimitiveComponent.SetSimulatePhysics` (`self.Arrow_Stem`) true)
  (`PrimitiveComponent.AddImpulse` (`self.Arrow_Stem`) (* (`SceneComponent.GetForwardVector` (`self.Arrow_Stem`)) (`self.MagnusPowerStrengthMeter`)) "None" false))

(fn `UserConstructionScript`
  (`PrimitiveComponent.SetCenterOfMass` (`self.Arrow_Stem`) (`SceneComponent.RelativeLocation` (`self.CenterOfMass`)) "None"))