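; BasicWeapon is a mountable weapon pawn that the player rotates while possessing it and leaves with the mount action, repossessing ControllingPlayer.
; Move-right and horizontal look input yaw the actor by RotationSpeed, the latter marked as a mouse quick fix; vertical look pitches the controller.
; PossessionSphere overlaps toggle MainGameMode's hint text for MainCharacter.
; FireWeaponCD disarms and starts reload state; ReloadDelay prints a debug "bang!" and sets Reload after ReloadTime.
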(event `self.ReceivePossessed`
  (params (NewController :type "Controller Object Reference")))

(event `InputAxis|A_MoveRight`
  (params (AxisValue :type "Float (single-precision)"))
  (`self.K2_AddActorLocalRotation` (`KismetMathLibrary.MakeRotator` 0.0 0.0 (* AxisValue (`self.RotationSpeed`) (`GameplayStatics.GetWorldDeltaSeconds`)))))

(event `InputAction|A_Mount`
  (params (Key :type "Key Structure" :default "AnyKey"))
  ;[1 1 1] Unpossesing
  (:`Pressed`
    (`Controller.Possess` (`GameplayStatics.GetPlayerController` 0) (`self.ControllingPlayer`))))

(event `InputAxis|A_LookUp_Down`
  (params (AxisValue :type "Float (single-precision)"))
  ;[1 1 1] Rotation
  (`self.AddControllerPitchInput` AxisValue))

(event `self.ReceiveTick`
  (params (DeltaSeconds :type "Float (single-precision)")))

(event `InputAxis|A_LookRight_Left`
  (params (AxisValue :type "Float (single-precision)"))
  ;[1 1 1] Rotation
  ;[1 1 1] SQUARE DE LA SQUARES
  ;;[1 1 1] BIGGER SQUARE
  ;;;[1 1 1] **** QUICKFIX FOR MOUSE TO ROTATE WEAPONS ******
  (`self.K2_AddActorLocalRotation` (`KismetMathLibrary.MakeRotator` 0.0 0.0 (* AxisValue (`self.RotationSpeed`) (`GameplayStatics.GetWorldDeltaSeconds`)))))

(event `ReloadDelay`
  ;[1 1 1] Handle reload time
  (`KismetSystemLibrary.PrintString` "bang!")
  (`KismetSystemLibrary.Delay` (`self.ReloadTime`))
  (set `self.Reload` true))

(event `self.PossessionSphere.OnComponentBeginOverlap`
  (params (OverlappedComponent :type "PrimitiveComponent Object Reference") (OtherActor :type "Actor Object Reference") (OtherComp :type "PrimitiveComponent Object Reference") (OtherBodyIndex :type Integer) (bFromSweep :type Boolean) (SweepResult :type "HitResult Structure (by ref)"))
  ;[1 1 1] Trigger Hint Text
  (cast `/Game/Blueprints/MainCharacter` OtherActor)
  (bind _asmain_game_mode (cast `/Game/Blueprints/MainGameMode` (`GameplayStatics.GetGameMode`)))
  (`Widget.SetVisibility` (`/Game/Blueprints/MainGameMode.HintText` _asmain_game_mode) "Visible"))

(event `self.PossessionSphere.OnComponentEndOverlap`
  (params (OverlappedComponent :type "PrimitiveComponent Object Reference") (OtherActor :type "Actor Object Reference") (OtherComp :type "PrimitiveComponent Object Reference") (OtherBodyIndex :type Integer))
  ;[1 1 1] Trigger Hint Text
  (cast `/Game/Blueprints/MainCharacter` OtherActor)
  (bind _asmain_game_mode (cast `/Game/Blueprints/MainGameMode` (`GameplayStatics.GetGameMode`)))
  (`Widget.SetVisibility` (`/Game/Blueprints/MainGameMode.HintText` _asmain_game_mode) "Hidden"))

(fn `FireWeaponCD`
  ;[1 1 1] Tell weapon that it's time to reload
  (set `self.Reload` true)
  (set `self.Curr_Reload_CD` (`self.ReloadTime`))
  (set `self.IsArmed` false))

(fn `UserConstructionScript`)