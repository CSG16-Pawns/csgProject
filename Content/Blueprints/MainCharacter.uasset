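; Player character that walks and looks around, can switch to a top-down mode and can mount weapons by possessing them.
; Axis inputs drive look and movement, with control-rotation vectors flattened to the horizontal plane.
; SwitchMode possesses the game mode's TopDownPawn and unhides GridField actors; Mount possesses an overlapping BasicWeapon within its PossessionSphere and hides the hint text.
; The character registers itself as ControllingPlayer on weapons at BeginPlay and on top-down pawns when switching.
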(event `InputAction|SwitchMode`
  (params (Key :type "Key Structure" :default "AnyKey"))
  ;[1 1 1] Switch mode to top down
  (:`Pressed`
    (bind _asmain_game_mode (cast `/Game/Blueprints/MainGameMode` (`GameplayStatics.GetGameMode`)))
    (`Controller.Possess` (`GameplayStatics.GetPlayerController` 0) (`/Game/Blueprints/MainGameMode.TopDownPawn` _asmain_game_mode))
    (bind _outactors (`GameplayStatics.GetAllActorsOfClass` "/Game/Blueprints/TopDownPawn.TopDownPawn_C"))
    (for _array_element _outactors
      (set `/Game/Blueprints/TopDownPawn.ControllingPlayer` self _array_element)
      (bind _outactors_2 (`GameplayStatics.GetAllActorsOfClass` "/Game/Blueprints/GridField.GridField_C"))
      (for _array_element_2 _outactors_2
        (`self.SetActorHiddenInGame` _array_element_2 false)))))

(event `InputAxis|A_LookUp_Down`
  (params (AxisValue :type "Float (single-precision)"))
  ;[1 1 1] Rotation
  (`self.AddControllerPitchInput` AxisValue))

(event `InputAxis|A_MoveForward`
  (params (AxisValue :type "Float (single-precision)"))
  ;[1 1 1] Movement
  (`self.AddMovementInput` (`KismetMathLibrary.Normal` (`KismetMathLibrary.MakeVector` (.x (`KismetMathLibrary.GetForwardVector` (`self.GetControlRotation`))) (.y (`KismetMathLibrary.GetForwardVector` (`self.GetControlRotation`))))) AxisValue))

(event `self.ReceiveBeginPlay`
  ;[1 1 1] Initialize player variable for all weapons
  (bind _outactors (`GameplayStatics.GetAllActorsOfClass` "/Game/Blueprints/BasicWeapon.BasicWeapon_C"))
  (for _array_element _outactors
    (set `/Game/Blueprints/BasicWeapon.ControllingPlayer` self _array_element)))

(event `InputAxis|A_LookRight_Left`
  (params (AxisValue :type "Float (single-precision)"))
  ;[1 1 1] Rotation
  (`self.AddControllerYawInput` AxisValue))

(event `InputAxis|A_MoveRight`
  (params (AxisValue :type "Float (single-precision)"))
  ;[1 1 1] Movement
  (`self.AddMovementInput` (`KismetMathLibrary.Normal` (`KismetMathLibrary.MakeVector` (.x (`KismetMathLibrary.GetRightVector` (`self.GetControlRotation`))) (.y (`KismetMathLibrary.GetRightVector` (`self.GetControlRotation`))))) AxisValue))

(event `InputAction|A_Mount`
  (params (Key :type "Key Structure" :default "AnyKey"))
  (bind _item (`KismetArrayLibrary.Array_Get` (`PrimitiveComponent.GetOverlappingActors` (`self.CapsuleComponent`) "/Game/Blueprints/BasicWeapon.BasicWeapon_C")))
  ;[1 1 1] Possesing
  (:`Pressed`
    (`/Engine/EditorBlueprintResources/StandardMacros.IsValid` _item
      (:`Is Valid`
        (bind _asbasic_weapon (cast `/Game/Blueprints/BasicWeapon` _item))
        (if (`PrimitiveComponent.IsOverlappingComponent` (`self.CapsuleComponent`) (`/Game/Blueprints/BasicWeapon.PossessionSphere` _asbasic_weapon))
          (`Controller.Possess` (`GameplayStatics.GetPlayerController` 0) _asbasic_weapon)
          (bind _asmain_game_mode (cast `/Game/Blueprints/MainGameMode` (`GameplayStatics.GetGameMode`)))
          (`Widget.SetVisibility` (`/Game/Blueprints/MainGameMode.HintText` _asmain_game_mode) "Hidden"))))))

(fn `UserConstructionScript`)