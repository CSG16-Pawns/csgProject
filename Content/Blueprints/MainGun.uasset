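; MainGun is a mountable gun that the player can possess and aim, with no firing logic in its graphs.
; Look axes drive controller pitch and yaw, and the mount action hands possession back to the stored ControllingPlayer.
; Overlaps of MainCharacter with PossessionSphere show or hide the hint text held by MainGameMode.
; Taking possession of the gun is not handled here, only releasing it.
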(event `InputAction|A_Mount`
  (params (Key :type "Key Structure" :default "AnyKey"))
  ;[1 1 1] Unpossesing
  (:`Pressed`
    (`Controller.Possess` (`GameplayStatics.GetPlayerController` 0) (`self.ControllingPlayer`))))

(event `InputAxis|A_LookUp_Down`
  (params (AxisValue :type "Float (single-precision)"))
  ;[1 1 1] Rotation
  (`self.AddControllerPitchInput` AxisValue))

(event `InputAxis|A_LookRight_Left`
  (params (AxisValue :type "Float (single-precision)"))
  ;[1 1 1] Rotation
  (`self.AddControllerYawInput` AxisValue))

(event `self.PossessionSphere.OnComponentBeginOverlap`
  (params (OverlappedComponent :type "PrimitiveComponent Object Reference") (OtherActor :type "Actor Object Reference") (OtherComp :type "PrimitiveComponent Object Reference") (OtherBodyIndex :type Integer) (bFromSweep :type Boolean) (SweepResult :type "HitResult Structure (by ref)"))
  ;[1 1 1] Trigger Hint Text
  (cast `/Game/Blueprints/MainCharacter` OtherActor)
  (bind _asmain_game_mode (cast `/Game/Blueprints/MainGameMode` (`GameplayStatics.GetGameMode`)))
  (`Widget.SetVisibility` (`/Game/Blueprints/MainGameMode.HintText` _asmain_game_mode) "Visible"))

(event `self.PossessionSphere.OnComponentEndOverlap`
  (params (OverlappedComponent :type "PrimitiveComponent Object Reference") (OtherActor :type "Actor Object Reference") (OtherComp :type "PrimitiveComponent Object Reference") (OtherBodyIndex :type Integer))
  ;[1 1 1] Trigger Hint Text
  (cast `/Game/Blueprints/MainCharacter` OtherActor)
  (bind _asmain_game_mode (cast `/Game/Blueprints/MainGameMode` (`GameplayStatics.GetGameMode`)))
  (`Widget.SetVisibility` (`/Game/Blueprints/MainGameMode.HintText` _asmain_game_mode) "Hidden"))

(fn `UserConstructionScript`)