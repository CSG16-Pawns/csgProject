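; MoveGroupActor_Panda is a movable actor that glides toward a TargetLocation, initialized to its spawn position on BeginPlay.
; Each Tick offsets it without sweep, at a fixed step when far away and a proportional ease-out when near, independent of delta time.
; The SwitchMode input, labeled as unpossessing, makes player controller 0 possess player pawn 0.
; Nothing here changes the target after initialization.
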(event `InputAction|SwitchMode`
  (params (Key :type "Key Structure" :default "AnyKey"))
  ;[1 1 1] Unpossesing
  (:`Pressed`
    (`Controller.Possess` (`GameplayStatics.GetPlayerController` 0) (`GameplayStatics.GetPlayerPawn` 0))))

(event `self.ReceiveBeginPlay`
  ;[1 1 1] Initialize actor location
  (set `self.TargetLocation` (`self.K2_GetActorLocation`)))

(event `self.ReceiveTick`
  (params (DeltaSeconds :type "Float (single-precision)"))
  (bind _returnvalue (`self.K2_GetActorLocation`))
  (bind _targetlocation (`self.TargetLocation`))
  (bind _returnvalue_2 (- _targetlocation _returnvalue))
  ;[1 1 1] Movement
  (if (== _targetlocation _returnvalue :`ErrorTolerance` 1000.0)
    (`self.K2_AddActorWorldOffset` (/ _returnvalue_2 10))
    (else
      (`self.K2_AddActorWorldOffset` (* (`KismetMathLibrary.Normal` _returnvalue_2) 50)))))

(fn `UserConstructionScript`)